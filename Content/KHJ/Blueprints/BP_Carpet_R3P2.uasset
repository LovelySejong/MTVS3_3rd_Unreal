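; BP_Carpet_R3P2 is an actor that raises and lowers the first actor tagged "Quiz3", found at BeginPlay.
; GoingUp plays and GoingDown reverses a timeline that sets that actor's Z while pinning its X and Y to the carpet's.
; RepNotify flags IsGoingUp and IsGoingDown trigger those events.
; Their setter events are only bound to BP_HJCharacter in disconnected nodes, and one is marked unused.
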(event `self.ReceiveBeginPlay`
  (bind _outactors (`GameplayStatics.GetAllActorsWithTag` "Quiz3"))
  (set `self.Q3Actor` (`|GetArrayItem` _outactors)))

(event `GoingUp`
  (bind (_returnvalue_x _returnvalue_y) (`KismetMathLibrary.BreakVector` (`self.K2_GetActorLocation`)))
  (bind (_direction _goingdown) (`Timeline|Timeline` :!label _label)
    (:`Update`
      (`self.K2_SetActorLocation` (`self.Q3Actor`) (`KismetMathLibrary.MakeVector` _returnvalue_x _returnvalue_y _goingdown) false false))))

(event `CustomEvent`
  ;[1 1 1] 안 씀
  (set `self.bIsGoingUp` true))

(event `GoingDown`
  (goto _label :!via `Reverse`))

(event `CustomEvent_0`
  ;[1 1 1] 안 씀
  (set `self.IsGoingDown` true))

(fn `OnRep_bIsGoingUp`
  (`self.GoingUp`))

(fn `OnRep_IsGoingDown`
  (`self.GoingDown`))

(fn `UserConstructionScript`)