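; BP_Carpet is a carpet actor that raises or lowers the first actor tagged Quiz3, triggered by the player character.
; On BeginPlay it binds to BP_HJCharacter's up and down events, but only the up handler acts, setting IsActivate and printing debug text.
; The OnRep function calls GoingUp, whose Timeline drives that actor's Z location.
; GoingDown shares the same forward Timeline play, and the bound down handler is empty.
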(event `self.ReceiveBeginPlay`
  (`|ExecutionSequence`
    (:`then_0`
      (bind _asbp_hjcharacter (cast `/Game/KHJ/Blueprints/BP_HJCharacter` (`GameplayStatics.GetPlayerPawn` 0)))
      (add `/Game/KHJ/Blueprints/BP_HJCharacter.GoingUpEvent` _asbp_hjcharacter (delegate `CustomEvent`)))
    (:`then_1`
      (bind _asbp_hjcharacter_2 (cast `/Game/KHJ/Blueprints/BP_HJCharacter` (`GameplayStatics.GetPlayerPawn` 0)))
      (add `/Game/KHJ/Blueprints/BP_HJCharacter.GoingDownEvent` _asbp_hjcharacter_2 (delegate `CustomEvent_0`)))))

(event `GoingUp`
  (bind _outactors (`GameplayStatics.GetAllActorsWithTag` "Quiz3" :!label _label))
  (bind (_direction _goingdown) (`Timeline|Timeline`)
    (:`Update`
      (bind _output (`|GetArrayItem` _outactors))
      (bind (_returnvalue_x _returnvalue_y) (`KismetMathLibrary.BreakVector` (`self.K2_GetActorLocation` _output)))
      (`self.K2_SetActorLocation` _output (`KismetMathLibrary.MakeVector` _returnvalue_x _returnvalue_y _goingdown) false false))))

(event `CustomEvent`
  (set `self.bIsActivate` true)
  (`KismetSystemLibrary.PrintString` "Hello")
  (`KismetSystemLibrary.PrintString` (`KismetSystemLibrary.GetDisplayName` (`self.GetOwner`))))

(event `GoingDown`
  (goto _label))

(event `CustomEvent_0`)

(fn `OnRep_bIsActivate`
  (`self.GoingUp`))

(fn `UserConstructionScript`)