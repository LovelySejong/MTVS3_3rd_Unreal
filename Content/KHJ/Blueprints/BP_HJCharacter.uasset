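; BP_HJCharacter is a character Blueprint that gives the player a hint key and holds test logic for a lever puzzle.
; Pressing H calls UseHint, which is not defined in this graph.
; Two chains are unwired and never run: one creates and shows WBP_Hint, the other flip-flops success and failure for all four levers through BP_HJGameMode's CheckLever.
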(event `Key|Q`
  (params (Key :type "Key Structure"))
  ;[1 1 1] 레버 기믹 성공/실패
)

(event `Key|H`
  (params (Key :type "Key Structure"))
  (:`Pressed`
    (`self.UseHint`)))

(fn `UserConstructionScript`)