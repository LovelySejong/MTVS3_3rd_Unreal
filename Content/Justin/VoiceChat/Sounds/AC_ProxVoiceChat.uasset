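; Actor component that sets up proximity voice chat on the Character that owns it.
; On BeginPlay it adds a VOIPTalker to the character, then polls on a short delay until the PlayerState is valid to register the talker with it.
; It sets the mic threshold and spatializes the voice from the capsule using attenuation and effect chain assets.
; Locally controlled characters also enable voice loopback through a console command.
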(event `self.ReceiveBeginPlay`
  (bind _ascharacter (cast `Character` (`self.GetOwner`))
    (:`then`
      (bind _output_get (set `self.As Character` _ascharacter))
      (bind _returnvalue (`|AddComponentByClass` _output_get "/Script/Engine.VOIPTalker"))
      (set `self.VoiceChatComp` _returnvalue)
      (`/Engine/EditorBlueprintResources/StandardMacros.IsValid` (`Pawn.PlayerState` (`self.As Character`)) :!label _label
        (:`Is Valid`
          (`VOIPTalker.RegisterWithPlayerState` (`self.VoiceChatComp`) (`Pawn.PlayerState` (`self.As Character`)))
          (`VOIPStatics.SetMicThreshold` -1.0)
          (set `VOIPTalker.Settings` (make `VoiceSettings` (`Character.CapsuleComponent` (`self.As Character`)) "/Game/Justin/VoiceChat/Sounds/ATT_VoiceChat.ATT_VoiceChat" "/Game/Justin/VoiceChat/Sounds/SC_VoiceChat.SC_VoiceChat") (`self.VoiceChatComp`))
          (if (`Pawn.IsLocallyControlled` (`self.As Character`))
            (`KismetSystemLibrary.ExecuteConsoleCommand` "OSS.VoiceLoopback 1" null)))
        (:`Is Not Valid`
          (`KismetSystemLibrary.Delay` 0.2)
          (goto _label))))
    (:`CastFailed`
      (`KismetSystemLibrary.PrintString` "Failed to cast to character in BeginPlay in AC_ProxVoiceChat Actor Component"))))