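; BP_FishBoxButton is an interactable puzzle button that reveals a hidden dial pad when the fish count matches the answer.
; On BeginPlay it finds the BP_DialPad tagged with DialName.
; A correct Interact calls ServerInteract then MulticastInteract, playing an opening sound and sliding the dial into view with a Timeline; a wrong count plays an error sound.
; Cursor events toggle custom depth on the mesh for highlighting.
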(event `self.ReceiveBeginPlay`
  (bind _outactors (`GameplayStatics.GetAllActorsOfClassWithTag` "/Game/CSW/Blueprints/BP_DialPad.BP_DialPad_C" (`self.DialName`)))
  (for _array_element _outactors
    (`KismetSystemLibrary.PrintString` (`KismetSystemLibrary.GetDisplayName` _array_element))
    (bind _asbp_dial_pad (cast `/Game/CSW/Blueprints/BP_DialPad` (`|GetArrayItem` _outactors))
      (:`then`
        (set `self.HiddenDial` _asbp_dial_pad))
      (:`CastFailed`
        (`KismetSystemLibrary.PrintString` "Hello")))))

(event `ServerInteract`
  (`self.MulticastInteract`))

(event `self.Interact`
  (params (caller :type "MTVS3_3rdCharacter Object Reference"))
  (if (== (`self.Answer`) (`self.FishCnt`))
    (`self.ServerInteract`)
    (else
      (`GameplayStatics.PlaySound2D` "/Game/CSW/Sound/WrongSound_Cue.WrongSound_Cue" 1.0 1.0 0.0 null null))))

(event `MulticastInteract`
  (`GameplayStatics.PlaySoundAtLocation` "/Game/CSW/Sound/DockableOpen_Cue.DockableOpen_Cue" (`self.K2_GetActorLocation`) (struct) 1.0 1.0 0.0 null null null null)
  (bind (_direction _door) (`Timeline|Timeline`)
    (:`Update`
      (`self.K2_SetActorRelativeLocation` (`self.HiddenDial`) (`KismetMathLibrary.VLerp` (`self.DisappearLocation`) (`self.AppearLocation`) _door) false false))))

(event `self.OnCursor`
  (`PrimitiveComponent.SetRenderCustomDepth` (`self.StaticMesh`) true))

(event `self.OffCursor`
  (`PrimitiveComponent.SetRenderCustomDepth` (`self.StaticMesh`) false))

(fn `Set Fish Cnt`
  (params (NewParam :type Integer))
  (set `self.FishCnt` NewParam))

(fn `UserConstructionScript`)