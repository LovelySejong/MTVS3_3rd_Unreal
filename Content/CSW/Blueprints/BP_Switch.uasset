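; BP_Switch is an interactable toggle switch that unlocks a door.
; At BeginPlay it caches the first BP_Door tagged DoorTag.
; Interact prints the owner's name and toggles through ServerOn/ServerOff: On unlocks the door and plays a Timeline rotating the switch, while Off only reverses the animation without relocking.
; Cursor events toggle custom depth rendering on the body.
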(event `self.ReceiveBeginPlay`
  (bind _outactors (`GameplayStatics.GetAllActorsOfClassWithTag` "/Game/CSW/Blueprints/BP_Door.BP_Door_C" (`self.DoorTag`)))
  (bind _asbp_door (cast `/Game/CSW/Blueprints/BP_Door` (`|GetArrayItem` _outactors)))
  (set `self.Door` _asbp_door))

(event `On`
  (set `self.bOn` true)
  (`/Game/CSW/Blueprints/BP_Door.Unlock` (`self.Door`))
  (bind (_direction _door) (`Timeline|Timeline` :!label _label)
    (:`Update`
      (`SceneComponent.K2_SetRelativeRotation` (`self.Switch`) (`KismetMathLibrary.MakeRotator` (`KismetMathLibrary.Lerp` 40.0 -40.0 _door)) false false))))

(event `Off`
  (set `self.bOn` false)
  (goto _label :!via `Reverse`))

(event `ServerOff`
  (`self.Off`))

(event `ServerOn`
  (`self.On`))

(event `self.Interact`
  (params (caller :type "MTVS3_3rdCharacter Object Reference"))
  (`KismetSystemLibrary.PrintString` (`KismetSystemLibrary.GetDisplayName` (`self.GetOwner`)))
  (if (`self.bOn`)
    (`self.ServerOff`)
    (else
      (`self.ServerOn`))))

(event `self.OnCursor`
  (`PrimitiveComponent.SetRenderCustomDepth` (`self.Body`) true))

(event `self.OffCursor`
  (`PrimitiveComponent.SetRenderCustomDepth` (`self.Body`) false))

(fn `UserConstructionScript`)