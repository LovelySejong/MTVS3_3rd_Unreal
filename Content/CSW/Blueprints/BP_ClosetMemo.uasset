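; Interactable memo Blueprint that opens a WBP_Memo widget when a caller interacts with it.
; At BeginPlay, scene capture component F renders a one-off capture showing only StaticMesh.
; Interact creates and caches the widget on first use, adds it to the viewport, and switches the player to UI-only input with cursor shown.
; Cursor events toggle custom depth on StaticMesh1 for highlighting, with a debug print on hover.
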(event `self.ReceiveBeginPlay`
  (bind _f (`self.f`))
  (`SceneCaptureComponent.ShowOnlyComponent` _f (`self.StaticMesh`))
  (`SceneCaptureComponent2D.CaptureScene` _f))

(event `self.Interact`
  (params (caller :type "MTVS3_3rdCharacter Object Reference"))
  (bind _returnvalue (`Pawn.GetLocalViewingPlayerController` caller))
  (`/Engine/EditorBlueprintResources/StandardMacros.IsValid` (`self.Widget`)
    (:`Is Valid`
      _)
    (:`Is Not Valid`
      (bind _returnvalue_2 (`|CreateWidget` "/Game/CSW/Blueprints/UI/WBP_Memo.WBP_Memo_C" _returnvalue))
      (bind _output_get (set `self.Widget` _returnvalue_2))))
  (`WidgetBlueprintLibrary.SetInputMode_UIOnlyEx` _returnvalue _output_get)
  (set `PlayerController.bShowMouseCursor` true _returnvalue)
  (`UserWidget.AddToViewport` (`self.Widget`) 0))

(event `self.OnCursor`
  (`KismetSystemLibrary.PrintString` "Hello")
  (`PrimitiveComponent.SetRenderCustomDepth` (`self.StaticMesh1`) true))

(event `self.OffCursor`
  (`PrimitiveComponent.SetRenderCustomDepth` (`self.StaticMesh1`) false))

(fn `UserConstructionScript`)