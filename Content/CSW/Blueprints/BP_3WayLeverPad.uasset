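; BP_3WayLeverPad is a puzzle pad, apparently for three-way levers, that checks entered values against a stored answer.
; PutNumber writes a value at an index in MyAnswer and compares the whole array to Answer.
; A match calls the ServerRpc event, which casts the game state to BP_HJGameState and calls MovingUpCarpet.
; A mismatch prints each current entry as debug output.
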(event `ServerRpc`
  (bind _asbp_hjgame_state (cast `/Game/KHJ/Blueprints/BP_HJGameState` (`GameplayStatics.GetGameState`)))
  (`MTVS3_3rdGameState.MovingUpCarpet` _asbp_hjgame_state))

(fn `PutNumber`
  (params (Idx :type Integer) (Value :type Integer))
  (`KismetArrayLibrary.Array_Set` (`self.MyAnswer`) Idx Value)
  (if (`KismetArrayLibrary.Array_Identical` (`self.Answer`) (`self.MyAnswer`))
    (`self.ServerRpc`)
    (else
      (for _array_element (`self.MyAnswer`)
        (`KismetSystemLibrary.PrintString` (`KismetStringLibrary.Conv_IntToString` _array_element))))))

(fn `UserConstructionScript`)