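; Interactable three-position lever that serves as a child actor of BP_3WayLeverPad and highlights its body via custom depth under the cursor.
; Interact goes through a server event to a multicast that plays a timeline, lerping the switch's roll from its captured pitch toward the adjacent RotationArr entry.
; When the timeline finishes, it steps Value, reports it with its index to the pad, and reverses direction at either end.
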(event `self.ReceiveBeginPlay`
  (bind _asbp_3way_lever_pad (cast `/Game/CSW/Blueprints/BP_3WayLeverPad` (`self.GetParentActor`)))
  (set `self.Pad` _asbp_3way_lever_pad))

(event `self.Interact`
  (params (caller :type "MTVS3_3rdCharacter Object Reference"))
  (`self.ServerInteract`))

(event `MulticastInteract`
  (bind _value (`self.Value`))
  (bind _pad (`self.Pad`))
  (bind _value_2 (`self.Value`))
  (bind _idx (`self.Idx`))
  (bind (_relativerotation_roll _relativerotation_pitch) (`KismetMathLibrary.BreakRotator` (`SceneComponent.RelativeRotation` (`self.Switch`))))
  (set `self.Relative Rotation Y (Pitch)` _relativerotation_pitch)
  (bind (_direction _door) (`Timeline|Timeline` :!via `PlayFromStart`)
    (:`Update`
      (if (`self.bRight`)
        (`SceneComponent.K2_SetRelativeRotation` (`self.Switch`) (`KismetMathLibrary.MakeRotator` (`KismetMathLibrary.Lerp` (`self.Relative Rotation Y (Pitch)`) (`|GetArrayItem` (`self.RotationArr`) (+ (`self.Value`) 1)) _door)) false false)
        (else
          (`SceneComponent.K2_SetRelativeRotation` (`self.Switch`) (`KismetMathLibrary.MakeRotator` (`KismetMathLibrary.Lerp` (`self.Relative Rotation Y (Pitch)`) (`|GetArrayItem` (`self.RotationArr`) (- (`self.Value`) 1)) _door)) false false))))
    (:`Finished`
      (if (`self.bRight`)
        (bind _output_get (set `self.Value` (+ _value 1)))
        (`/Game/CSW/Blueprints/BP_3WayLeverPad.PutNumber` _pad _idx _value_2)
        (if (== _output_get 2)
          (set `self.bRight` false))
        (else
          (bind _output_get_2 (set `self.Value` (- _value 1)))
          (`/Game/CSW/Blueprints/BP_3WayLeverPad.PutNumber` _pad _idx _value_2)
          (if (== _output_get_2 0)
            (set `self.bRight` true)))))))

(event `ServerInteract`
  (`self.MulticastInteract`))

(event `Right`)

(event `self.OnCursor`
  (`PrimitiveComponent.SetRenderCustomDepth` (`self.Body`) true))

(event `self.OffCursor`
  (`PrimitiveComponent.SetRenderCustomDepth` (`self.Body`) false))

(fn `UserConstructionScript`)