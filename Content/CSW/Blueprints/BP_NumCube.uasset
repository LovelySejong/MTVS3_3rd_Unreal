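; BP_NumCube is an interactable cube actor that highlights under the cursor and passes interactions to InteractCube along with the caller.
; On BeginPlay its SceneCaptureComponent2D takes a capture limited to the static mesh.
; Tick rotates the spring arm by scaled X and Y values as pitch and yaw.
; Cursor enter and exit events toggle the mesh's custom depth rendering.
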(event `self.ReceiveBeginPlay`
  (bind _scenecapturecomponent2d (`self.SceneCaptureComponent2D`))
  (`SceneCaptureComponent.ShowOnlyComponent` _scenecapturecomponent2d (`self.StaticMesh`))
  (`SceneCaptureComponent2D.CaptureScene` _scenecapturecomponent2d))

(event `self.ReceiveTick`
  (params (DeltaSeconds :type "Float (single-precision)"))
  (`SceneComponent.K2_AddLocalRotation` (`self.SpringArm`) (`KismetMathLibrary.MakeRotator` 0.0 (* (`self.Y`) 5.0) (* (`self.X`) 5.0)) false false))

(event `self.OnCursor`
  (`PrimitiveComponent.SetRenderCustomDepth` (`self.StaticMesh`) true))

(event `self.OffCursor`
  (`PrimitiveComponent.SetRenderCustomDepth` (`self.StaticMesh`) false))

(event `self.Interact`
  (params (caller :type "MTVS3_3rdCharacter Object Reference"))
  (`self.InteractCube` caller))

(fn `UserConstructionScript`)