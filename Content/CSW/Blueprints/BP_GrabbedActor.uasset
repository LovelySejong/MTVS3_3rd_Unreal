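; BP_GrabbedActor is an interactable actor that a caller can grab, hold in front of its first-person camera and release.
; Interact and InteractEnd toggle the grabbed state and switch mesh gravity through Server-to-Multicast events.
; While grabbed, Tick sets the actor's transform each frame to a fixed distance along the camera's forward vector.
; Cursor hover events toggle custom depth rendering on the mesh.
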(event `MulticastEvent`)

(event `self.ReceiveTick`
  (params (DeltaSeconds :type "Float (single-precision)"))
  (bind _firstpersoncameracomponent (`MTVS3_3rdCharacter.FirstPersonCameraComponent` (`self.Caller`)))
  (if (`self.IsGrabbed`)
    (`self.K2_SetActorLocationAndRotation` (+ (`SceneComponent.K2_GetComponentLocation` _firstpersoncameracomponent) (* (`SceneComponent.GetForwardVector` _firstpersoncameracomponent) 150.0)))))

(event `ServerEvent`
  (`self.MulticastEvent`))

(event `self.OnCursor`
  (`PrimitiveComponent.SetRenderCustomDepth` (`self.StaticMesh`) true))

(event `self.OffCursor`
  (`PrimitiveComponent.SetRenderCustomDepth` (`self.StaticMesh`) false))

(event `MulticastEnableGravity`
  (`PrimitiveComponent.SetEnableGravity` (`self.StaticMesh`) true))

(event `MulticastDisableGravity`
  (`PrimitiveComponent.SetEnableGravity` (`self.StaticMesh`) false))

(event `self.Interact`
  (params (caller :type "MTVS3_3rdCharacter Object Reference"))
  (set `self.Caller` caller)
  (set `self.IsGrabbed` true)
  (`self.ServerDisableGravity`))

(event `ServerEnableGravity`
  (`self.MulticastEnableGravity`))

(event `self.InteractEnd`
  (set `self.IsGrabbed` false)
  (`self.ServerEnableGravity`))

(event `ServerDisableGravity`
  (`self.MulticastDisableGravity`))

(fn `UserConstructionScript`)