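; BP_DialNumber is a single number key that lives as a child actor of a BP_DialPad, which it caches from its parent actor on BeginPlay.
; Cursor events toggle custom depth rendering on its mesh as a hover highlight.
; Interact routes through ServerInteract to MulticastInteract, which passes the key's Number to the pad's PutNumber.
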(event `self.ReceiveBeginPlay`
  (bind _asbp_dial_pad (cast `/Game/CSW/Blueprints/BP_DialPad` (`self.GetParentActor`)))
  (set `self.Pad` _asbp_dial_pad))

(event `self.ReceiveTick`
  (params (DeltaSeconds :type "Float (single-precision)")))

(event `self.OnCursor`
  (`PrimitiveComponent.SetRenderCustomDepth` (`self.StaticMesh`) true))

(event `self.OffCursor`
  (`PrimitiveComponent.SetRenderCustomDepth` (`self.StaticMesh`) false))

(event `ServerInteract`
  (`self.MulticastInteract`))

(event `self.Interact`
  (params (caller :type "MTVS3_3rdCharacter Object Reference"))
  (`self.ServerInteract`))

(event `MulticastInteract`
  (`/Game/CSW/Blueprints/BP_DialPad.PutNumber` (`self.Pad`) (`self.number`)))

(fn `UserConstructionScript`)