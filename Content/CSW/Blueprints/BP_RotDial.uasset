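; BP_RotDial is an interactable eight-position dial that belongs to a parent BP_RotDialPad, cached on BeginPlay.
; Cursor hover toggles custom depth on its mesh.
; Interact passes through server and multicast events, then a timeline rolls the mesh 45 degrees from its current rotation.
; When the timeline finishes, the dial increments its wrapping value and reports it with its index to the pad.
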(event `self.ReceiveBeginPlay`
  (bind _asbp_rot_dial_pad (cast `/Game/CSW/Blueprints/BP_RotDialPad` (`self.GetParentActor`)))
  (set `self.Pad` _asbp_rot_dial_pad))

(event `self.OnCursor`
  (`PrimitiveComponent.SetRenderCustomDepth` (`self.StaticMesh`) true))

(event `self.OffCursor`
  (`PrimitiveComponent.SetRenderCustomDepth` (`self.StaticMesh`) false))

(event `self.Interact`
  (params (caller :type "MTVS3_3rdCharacter Object Reference"))
  (`self.ServerInteract`))

(event `ServerInteract`
  (`self.MulticastInteract`))

(event `MulticastInteract`
  (bind _relative_rotation_x__roll_ (`self.Relative Rotation X (Roll)`))
  (bind _relativerotation_roll (`KismetMathLibrary.BreakRotator` (`SceneComponent.RelativeRotation` (`self.StaticMesh`))))
  (set `self.Relative Rotation X (Roll)` _relativerotation_roll)
  (bind (_direction _door) (`Timeline|Timeline` :!via `PlayFromStart`)
    (:`Update`
      (`SceneComponent.K2_SetRelativeRotation` (`self.StaticMesh`) (`KismetMathLibrary.MakeRotator` (`KismetMathLibrary.Lerp` _relative_rotation_x__roll_ (+ _relative_rotation_x__roll_ 45.0) _door)) false false))
    (:`Finished`
      (bind _output_get (set `self.Value` (mod (+ (`self.Value`) 1) 8)))
      (`/Game/CSW/Blueprints/BP_RotDialPad.PutNumber` (`self.Pad`) (`self.Idx`) _output_get))))

(fn `UserConstructionScript`)