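; BP_FishBox is an actor that tracks how many BP_Fish actors are inside its capsule volume.
; On BeginPlay it caches its child actor as a BP_FishBoxButton reference.
; Capsule overlap begin and end events raise or lower the fish count and push the new value to the button's own count.
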(event `self.ReceiveBeginPlay`
  (bind _asbp_fish_box_button (cast `/Game/CSW/Blueprints/BP_FishBoxButton` (`ChildActorComponent.ChildActor` (`self.ChildActor`))))
  (set `self.Btn` _asbp_fish_box_button))

(event `self.Capsule.OnComponentBeginOverlap`
  (params (OverlappedComponent :type "PrimitiveComponent Object Reference") (OtherActor :type "Actor Object Reference") (OtherComp :type "PrimitiveComponent Object Reference") (OtherBodyIndex :type Integer) (bFromSweep :type Boolean) (SweepResult :type "HitResult Structure (by ref)"))
  (cast `/Game/CSW/Blueprints/BP_Fish` OtherActor)
  (bind _result (`/Engine/EditorBlueprintResources/StandardMacros.IncrementInt` (`self.FishCnt`))
    (:`  `
      (set `/Game/CSW/Blueprints/BP_FishBoxButton.FishCnt` _result (`self.Btn`)))))

(event `self.Capsule.OnComponentEndOverlap`
  (params (OverlappedComponent :type "PrimitiveComponent Object Reference") (OtherActor :type "Actor Object Reference") (OtherComp :type "PrimitiveComponent Object Reference") (OtherBodyIndex :type Integer))
  (cast `/Game/CSW/Blueprints/BP_Fish` OtherActor)
  (bind _result (`/Engine/EditorBlueprintResources/StandardMacros.DecrementInt` (`self.FishCnt`))
    (:`  `
      (set `/Game/CSW/Blueprints/BP_FishBoxButton.FishCnt` _result (`self.Btn`)))))

(fn `UserConstructionScript`)