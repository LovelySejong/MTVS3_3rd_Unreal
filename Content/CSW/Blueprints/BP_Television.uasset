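; BP_Television is an interactable TV that steps through screen materials and opens two doors once its counter reaches three, then ignores further interaction.
; Interact calls a server event that multicasts the turn-on sound, counter increment, material swap and door unlock.
; BeginPlay caches the left and right BP_Door actors from the first two results of a tag search.
; Cursor events toggle custom depth rendering for highlighting.
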(event `self.ReceiveBeginPlay`
  (bind _outactors (`GameplayStatics.GetAllActorsWithTag` (`self.DoorTag`)))
  (bind _asbp_door (cast `/Game/CSW/Blueprints/BP_Door` (`|GetArrayItem` _outactors)))
  (set `self.leftDoor` _asbp_door)
  (bind _asbp_door_2 (cast `/Game/CSW/Blueprints/BP_Door` (`|GetArrayItem` _outactors 1)))
  (set `self.RightDoor` _asbp_door_2))

(event `MulticastInteraction`
  (bind _rightdoor (`self.RightDoor`))
  (`GameplayStatics.PlaySoundAtLocation` "/Game/CSW/Sound/TvTurnOn_Cue.TvTurnOn_Cue" (`self.K2_GetActorLocation`) (struct) 1.0 1.0 0.0 null null null null)
  (bind _result (`/Engine/EditorBlueprintResources/StandardMacros.IncrementInt` (`self.Idx`))
    (:`  `
      (if (== _result 3)
        (`/Game/CSW/Blueprints/BP_Door.Unlock` _rightdoor)
        (`/Game/CSW/Blueprints/BP_Door.Unlock` (`self.leftDoor`))
        (`/Game/CSW/Blueprints/BP_Door.ServerOpen` _rightdoor)
        (`/Game/CSW/Blueprints/BP_Door.ServerOpen` (`self.leftDoor`)))
      (`PrimitiveComponent.SetMaterial` (`self.StaticMesh1`) 0 (`|GetArrayItem` (`self.Material`) _result)))))

(event `ServerInteraction`
  (`self.MulticastInteraction`))

(event `self.Interact`
  (params (caller :type "MTVS3_3rdCharacter Object Reference"))
  (if (not (== (`self.Idx`) 3))
    (`self.ServerInteraction`)))

(event `self.OnCursor`
  (`PrimitiveComponent.SetRenderCustomDepth` (`self.StaticMesh`) true))

(event `self.OffCursor`
  (`PrimitiveComponent.SetRenderCustomDepth` (`self.StaticMesh1`) false))

(fn `UserConstructionScript`)