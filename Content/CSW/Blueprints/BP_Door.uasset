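; BP_Door is an interactable, lockable door that swings open and closed.
; Interact, when unlocked, toggles it through ServerOpen or ServerClose, which play or reverse a timeline that lerps the door's yaw through a quarter turn.
; Unlock clears the lock, and cursor events toggle custom depth rendering on the door.
; The rotation OnRep function is empty.
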(event `self.ReceiveBeginPlay`)

(event `self.ReceiveTick`
  (params (DeltaSeconds :type "Float (single-precision)")))

(event `Open`
  (set `self.bOpen` true)
  (bind (_direction _door) (`Timeline|OpenTimeline` :!label _label)
    (:`Update`
      (`SceneComponent.K2_SetRelativeRotation` (`self.Door`) (`KismetMathLibrary.MakeRotator` 0.0 0.0 (`KismetMathLibrary.Lerp` 0.0 -90.0 _door)) false false))))

(event `Close`
  (set `self.bOpen` false)
  (goto _label :!via `Reverse`))

(event `ServerClose`
  (`self.Close`))

(event `self.Interact`
  (params (caller :type "Object Object Reference"))
  (`KismetSystemLibrary.PrintString` (`KismetSystemLibrary.GetDisplayName` (`self.GetOwner`)))
  (if (not (`self.bLock`))
    (if (`self.bOpen`)
      (`self.ServerClose`)
      (else
        (`self.ServerOpen`)))))

(event `ServerOpen`
  (`self.Open`))

(event `self.OnCursor`
  (`PrimitiveComponent.SetRenderCustomDepth` (`self.Door`) true))

(event `self.OffCursor`
  (`PrimitiveComponent.SetRenderCustomDepth` (`self.Door`) false))

(fn `OnRep_RepliRotation`)

(fn `Unlock`
  (set `self.bLock` false))

(fn `UserConstructionScript`)