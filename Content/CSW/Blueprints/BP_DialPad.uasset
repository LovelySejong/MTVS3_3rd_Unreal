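; BP_DialPad is a keypad that unlocks a BP_Door when the entered code matches its Answer.
; On BeginPlay it caches the WBP_DialScreen from its widget component and the first BP_Door tagged DoorTag.
; PutNumber appends digits to the screen text, treating -2 as submit and -1 as clear; a wrong submission also clears the entry.
; A separate Cancel function empties the stored entry without refreshing the screen.
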(event `self.ReceiveBeginPlay`
  (bind _aswbp_dial_screen (cast `/Game/CSW/Blueprints/UI/WBP_DialScreen` (`WidgetComponent.GetWidget` (`self.Widget`))))
  (set `self.As WBP Dial Screen` _aswbp_dial_screen)
  (bind _outactors (`GameplayStatics.GetAllActorsOfClassWithTag` "/Game/CSW/Blueprints/BP_Door.BP_Door_C" (`self.DoorTag`)))
  (bind _asbp_door (cast `/Game/CSW/Blueprints/BP_Door` (`|GetArrayItem` _outactors)))
  (set `self.Door` _asbp_door))

(event `self.ReceiveTick`
  (params (DeltaSeconds :type "Float (single-precision)")))

(fn `Cancel`
  (set `self.MyAnswer` ""))

(fn `PutNumber`
  (params (NewParam :type Integer))
  (bind _textblock (`/Game/CSW/Blueprints/UI/WBP_DialScreen.TextBlock` (`self.As WBP Dial Screen`)))
  (switch `int` NewParam
    (:`Default`
      (bind _output_get (set `self.MyAnswer` (`KismetStringLibrary.Concat_StrStr` (`self.MyAnswer`) (`KismetStringLibrary.Conv_IntToString` NewParam))))
      (set `TextBlock.Text` (`KismetTextLibrary.Conv_StringToText` _output_get) _textblock))
    (:`-2`
      (if (`KismetStringLibrary.EqualEqual_StrStr` (`self.Answer`) (`self.MyAnswer`))
        (`/Game/CSW/Blueprints/BP_Door.Unlock` (`self.Door`))
        (else
          (bind _output_get_2 (set `self.MyAnswer` "" :!label _label))
          (set `TextBlock.Text` (`KismetTextLibrary.Conv_StringToText` _output_get_2) _textblock))))
    (:`-1`
      (goto _label))))

(fn `UserConstructionScript`)