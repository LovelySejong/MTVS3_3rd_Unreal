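; BP_KMJPlayer_2 is a player character Blueprint with a modular skeletal body and a hint input.
; The construction script makes the body, legs, feet, face and torso meshes follow the main mesh's pose.
; BeginPlay creates the WBP_Player widget without a local-control check, then activates post-processing only for the locally controlled player.
; Pressing H calls UseHint, whose logic lies outside these graphs.
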(event `self.ReceiveBeginPlay`
  (bind _returnvalue (`|CreateWidget` "/Game/CSW/Blueprints/UI/WBP_Player.WBP_Player_C"))
  (`UserWidget.AddToViewport` _returnvalue 0)
  (if (`self.IsLocallyControlled`)
    (`ActorComponent.Activate` (`self.PostProcess`) false)
    (else
      (`ActorComponent.Deactivate` (`self.PostProcess`)))))

(event `Key|H`
  (params (Key :type "Key Structure"))
  (:`Pressed`
    (`self.UseHint`)))

(fn `UserConstructionScript`
  (`SkinnedMeshComponent.SetLeaderPoseComponent` (`self.Body`) (`self.Mesh`) false false)
  (`SkinnedMeshComponent.SetLeaderPoseComponent` (`self.Legs`) (`self.Mesh`) false false)
  (`SkinnedMeshComponent.SetLeaderPoseComponent` (`self.Feet`) (`self.Mesh`) false false)
  (`SkinnedMeshComponent.SetLeaderPoseComponent` (`self.Face`) (`self.Mesh`) false false)
  (`SkinnedMeshComponent.SetLeaderPoseComponent` (`self.Torso`) (`self.Mesh`) false false))